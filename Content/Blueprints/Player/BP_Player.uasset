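; First-person player that walks and interacts while wandering, and carries the food, hunger and status rules for a round-based survival game.
; Enhanced Input drives movement and look, gated by CanMove, which follows the GameManager state at start.
; A camera line trace ignoring "Prop"-tagged actors toggles the reticle each tick and, on interact, collects items or calls BPI_Interactable.
; EatFood maps food attributes to GameManager stat changes, sounds and poison or infection counters, which ApplyStatus counts down.
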(event `self.ReceiveBeginPlay`
  (bind _outactors (`GameplayStatics.GetAllActorsWithTag` "Prop"))
  (set `self.IgnoreActors` _outactors)
  (`self.InitializeInput`)
  (`KismetSystemLibrary.DelayUntilNextTick`)
  (if (`|EnumEquality` (`GameManager.CurrentState` (`self.gameManager`)) "Wandering")
    (set `self.CanMove` true)
    (`/Engine/EditorBlueprintResources/StandardMacros.IsValid` (`self.MusicRef`)
      (:`Is Not Valid`
        (bind _returnvalue (`AddComponent|NODE_AddAudioComponent-5`))
        (set `self.MusicRef` _returnvalue)))
    (else
      (set `self.CanMove` false)
      (`/Engine/EditorBlueprintResources/StandardMacros.IsValid` (`self.MusicRef`)
        (:`Is Not Valid`
          (bind _returnvalue_2 (`AddComponent|NODE_AddAudioComponent-7`))
          (set `self.MusicRef` _returnvalue_2))))))

(event `self.ReceiveTick`
  (params (DeltaSeconds :type "Float (single-precision)"))
  (bind (_returnvalue _outhit) (`self.RaycastForward`))
  (bind (_bblockinghit _binitialoverlap _time _distance _location _impactpoint _normal _impactnormal _physmat _hitactor) (`GameplayStatics.BreakHitResult` _outhit))
  (`/Engine/EditorBlueprintResources/StandardMacros.IsValid` _hitactor
    (:`Is Valid`
      (cast `/Game/Blueprints/Core/BPI_Interactable` _hitactor
        (:`then`
          (`self.OnShowReticle`))
        (:`CastFailed`
          (`self.OnHideReticle`))))))

(event `EnhancedInput|/Game/Blueprints/Player/Input/Actions/IA_Move`
  (params (ActionValue :type "Vector2D Structure") (ElapsedSeconds :type "Float (double-precision)") (TriggeredSeconds :type "Float (double-precision)") (InputAction :type "InputAction Object Reference" :default "/Game/Blueprints/Player/Input/Actions/IA_Move.IA_Move"))
  (bind _movespeed (`self.MoveSpeed`))
  (:`Triggered`
    (if (`self.CanMove`)
      (`self.AddMovementInput` (`self.GetActorForwardVector`) (* ActionValue_Y _movespeed))
      (`self.AddMovementInput` (`self.GetActorRightVector`) (* ActionValue_X _movespeed)))))

(event `EnhancedInput|/Game/Blueprints/Player/Input/Actions/IA_MouseLook`
  (params (ActionValue :type "Vector2D Structure") (ElapsedSeconds :type "Float (double-precision)") (TriggeredSeconds :type "Float (double-precision)") (InputAction :type "InputAction Object Reference" :default "/Game/Blueprints/Player/Input/Actions/IA_MouseLook.IA_MouseLook"))
  (:`Triggered`
    (if (`self.CanMove`)
      (`self.AddControllerYawInput` ActionValue_X)
      (`self.AddControllerPitchInput` (* ActionValue_Y -1)))))

(event `EnhancedInput|/Game/Blueprints/Player/Input/Actions/IA_Interact`
  (params (ActionValue :type Boolean) (ElapsedSeconds :type "Float (double-precision)") (TriggeredSeconds :type "Float (double-precision)") (InputAction :type "InputAction Object Reference" :default "/Game/Blueprints/Player/Input/Actions/IA_Interact.IA_Interact"))
  (:`Started`
    (bind (_returnvalue _outhit) (`self.RaycastForward`))
    (bind (_bblockinghit _binitialoverlap _time _distance _location _impactpoint _normal _impactnormal _physmat _hitactor) (`GameplayStatics.BreakHitResult` _outhit))
    (if (`GameplayStatics.ObjectIsA` _hitactor "/Game/Blueprints/Items/BP_Item.BP_Item_C")
      (bind _asbp_item (cast `/Game/Blueprints/Items/BP_Item` _hitactor))
      (`GameManager.AddItems` (`self.GameManager`) _asbp_item))
    (bind _asbpi_interactable (cast `/Game/Blueprints/Core/BPI_Interactable` _hitactor))
    (`/Game/Blueprints/Core/BPI_Interactable.Interact` _asbpi_interactable)))

(fn `ApplyStatus`
  (if (> (`self.PoisonCounter`) 0)
    (`/Engine/EditorBlueprintResources/StandardMacros.DecrementInt` (`self.PoisonCounter`)
      (:`  `
        (`GameManager.DepleteHealth` (`self.GameManager`) 10))))
  (if (> (`self.InfectedCounter`) 0)
    (`/Engine/EditorBlueprintResources/StandardMacros.DecrementInt` (`self.InfectedCounter`)
      (:`  `
        (`GameManager.DepleteHunger` (`self.GameManager`) 5)))))

(fn `EatFood`
  (params (FoodItem :type "/Game/Blueprints/Food/BP_Food Object Reference"))
  (bind _gamemanager (`self.gameManager`))
  (`GameplayStatics.SpawnSound2D` "/Game/Blueprints/Audio/ScreamSecretsEat.ScreamSecretsEat" 1.0 (`KismetMathLibrary.RandomFloatInRange` 0.75 1.25) 0.0 null)
  (switch `/Game/Blueprints/Food/FoodAttribute` (`/Game/Blueprints/Food/BP_Food.Attribute` FoodItem)
    (:`NewEnumerator0`
      (`GameManager.RestoreHunger` _gamemanager 20)
      (set `self.NotifString` "The food leaves a foul taste")
      (`GameplayStatics.SpawnSound2D` "/Game/Blueprints/Audio/ScreamSecretsSuccess.ScreamSecretsSuccess" 1.0 1.0 0.0 null :!label _label))
    (:`NewEnumerator1`
      (`GameManager.RestoreHunger` _gamemanager 40)
      (set `self.NotifString` "The food is delicious! Double hunger restored")
      (goto _label))
    (:`NewEnumerator2`
      (`GameManager.RestoreHunger` _gamemanager 20)
      (`GameManager.RestoreHealth` _gamemanager 20)
      (set `self.NotifString` "The food is fresh! Health restored")
      (goto _label))
    (:`NewEnumerator3`
      (`GameManager.RestoreHunger` _gamemanager 0)
      (set `self.PoisonCounter` 3)
      (set `self.NotifString` "Your stomach turns and poisoning sets in")
      (`GameplayStatics.SpawnSound2D` "/Game/Blueprints/Audio/ScreamSecretsFailure.ScreamSecretsFailure" 0.55 1.0 0.0 null :!label _label_2))
    (:`NewEnumerator4`
      (`GameManager.RestoreHunger` _gamemanager 20)
      (`GameManager.DepleteHealth` _gamemanager 20)
      (set `self.NotifString` "Hidden nails cause your mouth to bleed")
      (goto _label_2))
    (:`NewEnumerator5`
      (`GameManager.RestoreHunger` _gamemanager 20)
      (`GameManager.DepleteHealth` _gamemanager 20)
      (set `self.NotifString` "Broken glass lacerates your throat")
      (goto _label_2))
    (:`NewEnumerator6`
      (if (not (`self.TakenAntacid`))
        (`GameManager.DepleteHunger` _gamemanager 30)
        (set `self.NotifString` "The food is horrendous. You throw up onto the table")
        (goto _label_2)))
    (:`NewEnumerator7`
      (`GameManager.RestoreHunger` _gamemanager 20)
      (set `self.InfectedCounter` 3)
      (set `self.NotifString` "Something has gotten into your body. Food drain increased")
      (goto _label_2))))

(fn `InitializeInput`
  (bind _asplayer_con (cast `PlayerCon` (`self.GetController`)))
  (`EnhancedInputSubsystemInterface.AddMappingContext` (pcsubsystem `EnhancedInputLocalPlayerSubsystem` _asplayer_con) "/Game/Blueprints/Player/Input/IMC_Wander.IMC_Wander" 0 (struct)))

(fn `InitializeWandering`
  (bind _returnvalue (`|CreateWidget` "/Game/Blueprints/UI/UI_Reticle.UI_Reticle_C"))
  (`UserWidget.AddToViewport` _returnvalue 0)
  (set `self.CanMove` true))

(fn `PassRound`
  (`GameManager.DepleteHunger` (`self.GameManager`) 20))

(fn `UserConstructionScript`)