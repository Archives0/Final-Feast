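; BP_Item is a pickup item actor that can be filled with content and removed when the player interacts with it.
; SpawnItem sets its type, mesh, icon and description, then shows the mesh and enables its collision.
; Interact calls DespawnMesh, which clears the Spawned flag, hides the mesh and disables collision instead of destroying the actor, then plays a randomly pitched pickup sound.
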(event `/Game/Blueprints/Core/BPI_Interactable.Interact`
  (`self.DespawnMesh`)
  (`GameplayStatics.SpawnSound2D` "/Game/Blueprints/Audio/ScreamSecretsPickupItem.ScreamSecretsPickupItem" 1.0 (`KismetMathLibrary.RandomFloatInRange` 0.75 1.25) 0.0 null))

(fn `DespawnMesh`
  (bind _staticmesh (`self.StaticMesh`))
  (set `self.Spawned` false)
  (`SceneComponent.SetVisibility` _staticmesh false false)
  (`PrimitiveComponent.SetCollisionEnabled` _staticmesh "NoCollision"))

(fn `SpawnItem`
  (params (Mesh :type "StaticMesh Object Reference") (`UI Icon` :type "Texture2D Object Reference") (Type :type "EItemType Enum" :default "Milk") (Text :type String))
  (bind _staticmesh (`self.StaticMesh`))
  (set `self.Spawned` true)
  (set `self.ItemType` Type)
  (`StaticMeshComponent.SetStaticMesh` _staticmesh Mesh)
  (`SceneComponent.SetVisibility` _staticmesh true false)
  (`PrimitiveComponent.SetCollisionEnabled` _staticmesh "QueryAndPhysics")
  (set `self.Icon` `UI Icon`)
  (set `self.Description` Text))

(fn `UserConstructionScript`)